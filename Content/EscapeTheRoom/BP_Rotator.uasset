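; BP_Rotator is an actor that endlessly swings its Cube back and forth between two rotations.
; On BeginPlay it enables player input and calls Rotate, where a FlipFlop alternates playing and reversing a timeline that lerps the cube's relative rotation.
; The timeline's Finished pin calls Rotate again to sustain the loop.
; The C and D keys set the actor's custom time dilation to speed up or slow down the motion.
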(event Custom|Rotate
  (Utilities|FlowControl|FlipFlop
    (:A
      (bind _newtrack_0 (Timeline|Timeline_0 PlayFromStart)
        (:Update
          (Transformation|SetRelativeRotation (Variables|Default|GetCube) (Math|Rotator|Lerp(Rotator) (Variables|Default|Getrotation%201) (Variables|Default|Getrotation%202) _newtrack_0) false false))
        (:Finished
          (CallFunction|Rotate))))
    (:B
      (Timeline|Timeline_0 Reverse))))

(event EventBeginPlay
  (Input|EnableInput (Game|GetPlayerController 0))
  (CallFunction|Rotate))

(event Collision|EventActorBeginOverlap
  (params (OtherActor :type Actor%20Object%20Reference)))

(event Input|KeyboardEvents|C
  (params (Key :type Key%20Structure :default "None"))
  (:Pressed
    (Variables|Default|SetCustomTimeDilation 4.0)))

(event Input|KeyboardEvents|D
  (params (Key :type Key%20Structure :default "None"))
  (:Pressed
    (Variables|Default|SetCustomTimeDilation 0.1)))

(fn ConstructionScript)