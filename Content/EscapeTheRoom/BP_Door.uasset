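; Escape-room door that slides between its starting position and an offset, with unfinished logic to lock it until three keys are found.
; The Open/Close event alternates direction through a FlipFlop and MoveComponentTo, using a moving flag to block overlapping inputs.
; Key counting and the locked-door interaction check have no triggering events, so neither runs; comments suggest a cast or interface to connect them.
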(event Custom|Open/Close
  ;[1 1 1] This checks if the door is opening or closing so this process can stop before more inputs are accepted.
  (if (not (Variables|Default|GetIsmoving))
    (Variables|Default|SetIsmoving true)
    (Utilities|FlowControl|FlipFlop
      (:A
        (Components|MoveComponentTo (Variables|Default|GetDoor) (+ (Variables|Default|GetDoorLocation) (Variables|Default|GetDoorMovement)) "0, 0, 0" false false 0.2 false))
      (:B
        (Components|MoveComponentTo (Variables|Default|GetDoor) (Variables|Default|GetDoorLocation) "0, 0, 0" false false 0.2 false)))
    (Variables|Default|SetIsmoving false)))

(event EventBeginPlay
  (Variables|Default|SetDoorLocation (Variables|/Script/Engine.SceneComponent|GetRelativeLocation (Variables|Default|GetDoor))))

(fn ConstructionScript)