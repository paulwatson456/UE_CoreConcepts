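; BP_BoxSpawner is an Escape The Room actor that continuously spawns BP_BoxEnemy actors.
; On BeginPlay it caches the world locations of three spawn point components in an array and starts a looping two-second timer.
; Each timer tick spawns a box enemy at one of those locations, picked at random.
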(event Custom|BoxSpawner
  (Game|SpawnActorfromClass "/Game/EscapeTheRoom/BP_BoxEnemy.BP_BoxEnemy_C" (Math|Conversions|ToTransform(Vector) (Utilities|Array|Get(acopy) (Variables|Default|GetSpawn%20Locations) (Math|Random|RandomIntegerinRange 0 2))) "Undefined" 0 0))

(event EventBeginPlay
  (Utilities|Array|Add (Variables|Default|GetSpawn%20Locations) (Transformation|GetWorldLocation (Variables|Default|GetSpawnPoint3)))
  (Utilities|Array|Add (Variables|Default|GetSpawn%20Locations) (Transformation|GetWorldLocation (Variables|Default|GetSpawnPoint1)))
  (Utilities|Array|Add (Variables|Default|GetSpawn%20Locations) (Transformation|GetWorldLocation (Variables|Default|GetSpawnPoint2)))
  (Utilities|Time|SetTimerbyEvent (delegate Custom|BoxSpawner) 2.0 true))

(fn ConstructionScript)