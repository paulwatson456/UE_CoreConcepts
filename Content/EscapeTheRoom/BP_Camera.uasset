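; Escape-room camera actor that continuously sweeps its root component back and forth between roughly -89 and 89 degrees.
; BeginPlay starts RotateRight and RotateLeft, which call each other endlessly, each using MoveComponentTo for a timed turn followed by a short pause.
; An alternative Rotaate event, using a FlipFlop and the CameraRotation timeline to lerp the rotation, is left in the graph but never runs.
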(event Custom|rotate%20right
  (bind _defaultsceneroot (Variables|Default|GetDefaultSceneRoot))
  (Components|MoveComponentTo _defaultsceneroot (Transformation|GetWorldLocation _defaultsceneroot) "0,89.000000, 0" false false 4.0 false)
  (Utilities|FlowControl|Delay 1.0)
  (CallFunction|RotateLeft))

(event Custom|RotateLeft
  (Components|MoveComponentTo (Variables|Default|GetDefaultSceneRoot) (Transformation|GetWorldLocation (Variables|Default|GetDefaultSceneRoot)) "0,-89.000000, 0" false false 4.0 false)
  (Utilities|FlowControl|Delay 1.0)
  (CallFunction|RotateRight))

(event Custom|Rotaate
  (Utilities|FlowControl|FlipFlop
    (:A
      (bind _newtrack_0 (Timeline|CameraRotation PlayFromStart)
        (:Update
          (Transformation|SetWorldRotation (Variables|Default|GetDefaultSceneRoot) (Math|Rotator|Lerp(Rotator) "0,-90.000000, 0" "0,90.000000, 0" _newtrack_0) false false))
        (:Finished
          (CallFunction|Rotaate))))
    (:B
      (Timeline|CameraRotation ReverseFromEnd))))

(event EventBeginPlay
  (CallFunction|RotateRight))

(fn ConstructionScript)