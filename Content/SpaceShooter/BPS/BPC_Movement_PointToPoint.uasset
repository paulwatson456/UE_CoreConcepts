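; Movement component for a space shooter that flies its owning actor in a straight line from its BeginPlay location toward the average of the EndLOC points.
; Tick advances a normalized timer by TimeToCompleteSpline, lerps the position and wraps to the start, while aiming the X axis directly away from the player pawn.
; Events toggle movement and the flying flag, which IsFlyingCheck exposes; ExecuteFlightpath is an empty stub.
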(event Custom|ExecuteFlightpath)

(event EventBeginPlay
  (Variables|Default|SetStartLOC (Transformation|GetWorldLocation (Variables|/Script/Engine.Actor|GetRootComponent (Components|GetOwner))))
  (CallFunction|EnableMovement))

(event EventEnableMovement
  (Variables|Default|SetCanMove? true)
  (Variables|Default|SetIsFlying? true)
  (Variables|Default|SetZeroToOne 0.0))

(event EventStopMovement
  (Variables|Default|SetCanMove? false))

(event EventHasReturned?
  (Variables|Default|SetCanMove? false)
  (Variables|Default|SetIsFlying? false))

(event EventTick
  (params (DeltaSeconds :type Float%20%28single-precision%29))
  (bind _output_get (Variables|Default|SetZeroToOne (+ (/ DeltaSeconds (Variables|Default|GetTimeToCompleteSpline)) (Variables|Default|GetZeroToOne))))
  (if (> _output_get 1.0)
    (Variables|Default|SetZeroToOne 0.0))
  (if (Variables|Default|GetCanMove?)
    (Transformation|SetWorldLocationAndRotation (Variables|/Script/Engine.Actor|GetRootComponent (Components|GetOwner)) (Math|Vector|Lerp(Vector) (Variables|Default|GetStartLOC) (Math|Vector|GetVectorArrayAverage (Variables|Default|GetEndLOC)) (Variables|Default|GetZeroToOne)) (Math|Conversions|RotationFromXVector (- (Transformation|GetWorldLocation (Variables|/Script/Engine.Actor|GetRootComponent (Components|GetOwner))) (Transformation|GetActorLocation (Game|Player|GetPlayerPawn 0)))) false false)))

(fn IsFlyingCheck
  (return (Variables|Default|GetIsFlying?)))