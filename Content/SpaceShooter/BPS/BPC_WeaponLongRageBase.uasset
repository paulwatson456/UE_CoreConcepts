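; Base long-range weapon component that gives its owning actor an auto-firing hitscan gun in the space shooter.
; On BeginPlay it finds owner child components whose names contain the weapon type name, stores their relative location and starts firing.
; Fire re-calls itself after a multiplier-scaled delay, debug-drawing a line trace along world +X at Level 1.
; Blocking hits damage the actor through I_Entity_Damageable and spawn a Niagara impact.
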(event Custom|Fire
  (bind _returnvalue (Components|GetOwner))
  (bind _gunlocation (Variables|Default|GetGunLocation))
  (bind _rootcomponent (Variables|/Script/Engine.Actor|GetRootComponent _returnvalue))
  (bind _returnvalue_2 (Transformation|GetWorldLocation _rootcomponent))
  (bind _returnvalue_3 (+ _returnvalue_2 _gunlocation))
  (switch Utilities|FlowControl|Switch|SwitchonE_WeaponLevel (Variables|Default|GetPowerLevel)
    (:NewEnumerator0
      (bind _outhit (Collision|LineTraceByChannel _returnvalue_3 (+ _returnvalue_3 "1000.000000,0,0") "TraceTypeQuery1" false 0 "ForDuration" true "(R=1.000000,G=0.000000,B=0.000000,A=1.000000)" "(R=0.000000,G=1.000000,B=0.000000,A=1.000000)" (* (Variables|Default|GetFireRate) (Variables|Default|GetFireRateMultiplier))))
      (if (.bBlockingHit (Collision|BreakHitResult _outhit))
        (Class|IEntityDamageable|DamageEntityValue(Message) (Utilities|Array|Get(acopy) (Class|Actor|GetComponentsbyInterface (.HitActor (Collision|BreakHitResult _outhit)) "/Game/SpaceShooter/BPS/I_Entity_Damageable.I_Entity_Damageable_C")) (Variables|Default|GetDMG_BaseValue))
        (Niagara|SpawnSystematLocation "/Game/SpaceShooter/BPS/NS_GunImpact_01.NS_GunImpact_01" (.ImpactPoint (Collision|BreakHitResult _outhit))))
      (Utilities|FlowControl|Delay (* (Variables|Default|GetFireRate) (Variables|Default|GetFireRateMultiplier)))
      (CallFunction|Fire))))

(event EventBeginPlay
  (bind _weapontype (Variables|Default|GetWeaponType))
  (switch Utilities|FlowControl|Switch|SwitchonE_WeaponType _weapontype
    (:NewEnumerator0
      _)
    (:NewEnumerator1
      _)
    (:NewEnumerator2
      _))
  (Variables|Default|SetChosenWeaponTypeName (Utilities|Array|Get(acopy) (Variables|Default|GetWeaponTypeNames) (Math|Conversions|ToInteger(Byte) _weapontype)))
  (for _array_element (Components|GetChildrenComponents (Variables|/Script/Engine.Actor|GetRootComponent (Components|GetOwner)) true)
    (if (Utilities|String|Contains (Utilities|GetDisplayName _array_element) (Variables|Default|GetChosenWeaponTypeName))
      (Variables|Default|SetGunLocation (Variables|/Script/Engine.SceneComponent|GetRelativeLocation _array_element))
      (CallFunction|Fire))))