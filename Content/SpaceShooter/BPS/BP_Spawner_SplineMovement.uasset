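; Spawner actor for the space shooter that pre-spawns a pool of BP_EnemyMine_01 enemies and launches them one after another along a spline.
; On BeginPlay it fills EnemyPool at a fixed location, optionally enabling spline debug display first.
; ShipGO then adds a follow-spline movement component to each pooled enemy, passing the BPCSpawnSpline spline and travel time, and re-calls itself after SpawnRate until the pool is used up.
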(event Custom|ShipGO
  (if (not (> (Variables|Default|GetSpawnNumber) (Variables|Default|GetSpawnNumberMax)))
    (bind _returnvalue (AddComponent|AddBPCMovementFollowSpline (Utilities|Array|Get(acopy) (Variables|Default|GetEnemyPool) (Variables|Default|GetSpawnNumber))))
    (Variables|/Game/SpaceShooter/BPS/BPC_Movement_FollowSpline.BPC_Movement_FollowSpline_C|SetTimeToCompleteSpline _returnvalue (Variables|Default|GetTimeAcrossSpline))
    (Variables|/Game/SpaceShooter/BPS/BPC_Movement_FollowSpline.BPC_Movement_FollowSpline_C|SetSplineREF _returnvalue (Variables|/Game/SpaceShooter/BPS/BPC_SpawnSpline.BPC_SpawnSpline_C|GetSplineREF (Variables|Default|GetBPC_SpawnSpline)))
    (Utilities|FlowControl|Delay (Variables|Default|GetSpawnRate))
    (Variables|Default|SetSpawnNumber (+ (Variables|Default|GetSpawnNumber) 1))
    (CallFunction|ShipGO)))

(event Custom|Spawn%20and%20Pool
  (for _index (range 0 (Variables|Default|GetSpawnNumberMax))
    (bind _returnvalue (Game|SpawnActorfromClass "/Game/SpaceShooter/BPS/BP_EnemyMine_01.BP_EnemyMine_01_C" (Math|Transform|MakeTransform "0,1000.000000, 0" "0, 0, 0" "1.000000,1.000000,1.000000") "Undefined" 0 0))
    (Utilities|Array|Add (Variables|Default|GetEnemyPool) _returnvalue))
  (CallFunction|ShipGO))

(event EventBeginPlay
  (if (Variables|Default|GetDebugSplines?)
    (Development|ExecuteConsoleCommand "show splines" 0))
  (CallFunction|SpawnandPool))

(fn ConstructionScript)