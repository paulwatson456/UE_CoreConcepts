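; Gun component for the space shooter that makes its owner fire BP_Bullet_01 automatically and continuously.
; On BeginPlay it finds the owner's "GunPointMain" child component, stores its relative location and starts firing.
; TestFire picks a pattern by GunLevel: single, twin, or four shots with angled outer bullets, each looping back after a FireRate delay.
; The level-up increment logic is present but unconnected.
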(event Custom|TestFire
  (switch int (Variables|Default|GetGunLevel)
    (:Default
      (CallFunction|FireLVL1 :!label _label))
    (:0
      (goto _label))
    (:1
      (CallFunction|FireLVL2))
    (:2
      (CallFunction|FireLVL3))))

(event Custom|Set%20Gun%20Position
  (CallFunction|TestFire))

(event Custom|FireLVL_1
  (Game|SpawnActorfromClass "/Game/SpaceShooter/BPS/BP_Bullet_01.BP_Bullet_01_C" (Math|Conversions|ToTransform(Vector) (+ (Variables|Default|GetGunMainLocation) (Transformation|GetWorldLocation (Variables|/Script/Engine.Actor|GetRootComponent (Components|GetOwner))))) "Undefined" 0 0)
  (Utilities|FlowControl|Delay (Variables|Default|GetFireRate))
  (CallFunction|TestFire))

(event Custom|FireLVL_2
  (Game|SpawnActorfromClass "/Game/SpaceShooter/BPS/BP_Bullet_01.BP_Bullet_01_C" (Math|Conversions|ToTransform(Vector) (+ (+ (Variables|Default|GetGunMainLocation) (Transformation|GetWorldLocation (Variables|/Script/Engine.Actor|GetRootComponent (Components|GetOwner)))) "0.000000,-10.000000,0")) "Undefined" 0 0)
  (Game|SpawnActorfromClass "/Game/SpaceShooter/BPS/BP_Bullet_01.BP_Bullet_01_C" (Math|Conversions|ToTransform(Vector) (+ (+ (Variables|Default|GetGunMainLocation) (Transformation|GetWorldLocation (Variables|/Script/Engine.Actor|GetRootComponent (Components|GetOwner)))) "0.000000,10.000000,0")) "Undefined" 0 0)
  (Utilities|FlowControl|Delay (Variables|Default|GetFireRate))
  (CallFunction|TestFire))

(event Custom|FireLVL_3
  (Game|SpawnActorfromClass "/Game/SpaceShooter/BPS/BP_Bullet_01.BP_Bullet_01_C" (Math|Conversions|ToTransform(Vector) (+ (+ (Variables|Default|GetGunMainLocation) (Transformation|GetWorldLocation (Variables|/Script/Engine.Actor|GetRootComponent (Components|GetOwner)))) "0.000000,-10.000000,0")) "Undefined" 0 0)
  (Game|SpawnActorfromClass "/Game/SpaceShooter/BPS/BP_Bullet_01.BP_Bullet_01_C" (Math|Conversions|ToTransform(Vector) (+ (+ (Variables|Default|GetGunMainLocation) (Transformation|GetWorldLocation (Variables|/Script/Engine.Actor|GetRootComponent (Components|GetOwner)))) "0.000000,10.000000,0")) "Undefined" 0 0)
  (Game|SpawnActorfromClass "/Game/SpaceShooter/BPS/BP_Bullet_01.BP_Bullet_01_C" (Math|Transform|MakeTransform (+ (+ (Variables|Default|GetGunMainLocation) (Transformation|GetWorldLocation (Variables|/Script/Engine.Actor|GetRootComponent (Components|GetOwner)))) "0.000000,-20.000000,0") (Math|Rotator|MakeRotator 0.0 0.0 -5.0) "1.000000,1.000000,1.000000") "Undefined" 0 0)
  (Game|SpawnActorfromClass "/Game/SpaceShooter/BPS/BP_Bullet_01.BP_Bullet_01_C" (Math|Transform|MakeTransform (+ (+ (Variables|Default|GetGunMainLocation) (Transformation|GetWorldLocation (Variables|/Script/Engine.Actor|GetRootComponent (Components|GetOwner)))) "0.000000,20.000000,0") (Math|Rotator|MakeRotator 0.0 0.0 5.0) "1.000000,1.000000,1.000000") "Undefined" 0 0)
  (Utilities|FlowControl|Delay (Variables|Default|GetFireRate))
  (CallFunction|TestFire))

(event EventBeginPlay
  (bind _output_get (Variables|Default|SetOwnerChildren (Components|GetChildrenComponents (Variables|/Script/Engine.Actor|GetRootComponent (Components|GetOwner)) true)))
  (for (_array_element _array_index) _output_get
    (if (Utilities|String|Contains (Utilities|GetDisplayName _array_element) "GunPointMain")
      (Variables|Default|SetGunMainLocation (Variables|/Script/Engine.SceneComponent|GetRelativeLocation (Utilities|Array|Get(acopy) (Variables|Default|GetOwnerChildren) _array_index)))
      (Development|PrintString (Utilities|GetDisplayName (Utilities|Array|Get(acopy) (Variables|Default|GetOwnerChildren) _array_index)))
      (CallFunction|SetGunPosition))))

(event EventTick
  (params (DeltaSeconds :type Float%20%28single-precision%29)))