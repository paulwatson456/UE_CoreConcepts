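; Unused-folder Blueprint that rebuilds a spline track from saved points and tangents in a data asset, chosen by SplineSelection.
; The construction script builds the spline at SPMine01's relative location and prints a debug point.
; CreateSpline repeats the build at runtime, but nothing here calls it.
; BeginPlay and MoveObject are empty; the timeline logic for moving SPMine01 along the spline is disconnected.
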(event Custom|MoveObject)

(event Custom|CreateSpline
  (bind _splineselection (Variables|Default|GetSplineSelection))
  (bind _pda_splinetracks (Variables|Default|GetPDA_SplineTracks))
  (bind _st_splinetracks (Variables|/Game/SpaceShooter/BPS/SplineTracks/PDA_SplineTracks.PDA_SplineTracks_C|GetST_SplineTracks _pda_splinetracks))
  (bind _output (Utilities|Array|Get(acopy) _st_splinetracks _splineselection))
  ;[1 1 1] Creates Spline based on previously saved data
  (bind _returnvalue (AddComponent|AddSplineComponent false (Transformation|GetRelativeTransform (Variables|Default|GetDefaultSceneRoot))))
  (bind _output_get (Variables|Default|SetSplineTrackREF _returnvalue))
  (Spline|SetSplinePoints _output_get (.pointworldlocations _output) "Local" true)
  (for (_array_element _array_index) (.pointtangents _output)
    (Spline|SetTangentatSplinePoint (Variables|Default|GetSplineTrackREF) _array_index _array_element "Local" true))
  (CallFunction|MoveObject))

(event EventBeginPlay)

(fn ConstructionScript
  (bind _splineselection (Variables|Default|GetSplineSelection))
  (bind _pda_splinetracks (Variables|Default|GetPDA_SplineTracks))
  (bind _st_splinetracks (Variables|/Game/SpaceShooter/BPS/SplineTracks/PDA_SplineTracks.PDA_SplineTracks_C|GetST_SplineTracks _pda_splinetracks))
  (bind _output (Utilities|Array|Get(acopy) _st_splinetracks _splineselection))
  (bind _returnvalue (AddComponent|AddSplineComponent false (Math|Transform|MakeTransform (Variables|/Script/Engine.SceneComponent|GetRelativeLocation (Variables|Default|GetSP_Mine_01)) "0, 0, 0" "1.000000,1.000000,1.000000")))
  (bind _output_get (Variables|Default|SetSplineTrackREF _returnvalue))
  (Spline|SetSplinePoints _output_get (.pointworldlocations _output) "Local" false)
  (for (_array_element _array_index) (.pointtangents _output)
    (Spline|SetTangentatSplinePoint (Variables|Default|GetSplineTrackREF) _array_index _array_element "Local" false)
    (Development|PrintString (Utilities|String|ToString(Vector) (Utilities|Array|Get(acopy) (.pointworldlocations _output) 2)))))