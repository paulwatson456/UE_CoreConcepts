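; Base level director for a space shooter that spawns the player ship and in-game UI, then runs an enemy wave.
; Wave loading increments the wave number, briefly shows it on the UI and changes the ship's movement state.
; A squadron switch configures BP_SpawnerBase actors to send mines along selected splines.
; SquadrenDestroyed advances through three hard-coded squadrons, the last spawning two groups at once.
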(event Custom|LoadWave
  (bind _playershipref (Variables|Default|GetPlayerShipREF))
  (bind _result (Math|Integer|IncrementInt (Variables|Default|GetWaveNumber))
    (:%20%20
      (Variables|/Game/SpaceShooter/BPS/W_GUI.W_GUI_C|SetWaveNumberToDisplay (Variables|/Game/SpaceShooter/BPS/BP_InGame_UI.BP_InGame_UI_C|GetW_GUI_REF (Variables|Default|GetGUI_REF)) _result)
      (Default|ToggleWaveVisability (Variables|/Game/SpaceShooter/BPS/BP_InGame_UI.BP_InGame_UI_C|GetW_GUI_REF (Variables|Default|GetGUI_REF)))
      (Variables|/Game/SpaceShooter/BPS/P_Ship_01.P_Ship_01_C|SetPlayerMovementState (Variables|Default|GetPlayerShipREF) "NewEnumerator1")
      (Default|SetState _playershipref)
      (Variables|/Game/SpaceShooter/BPS/P_Ship_01.P_Ship_01_C|SetPlayerMovementState _playershipref "NewEnumerator3")
      (Default|SetState (Variables|Default|GetPlayerShipREF))
      (Utilities|FlowControl|Delay 2.0)
      (Default|ToggleWaveVisability (Variables|/Game/SpaceShooter/BPS/BP_InGame_UI.BP_InGame_UI_C|GetW_GUI_REF (Variables|Default|GetGUI_REF)))
      (CallFunction|SPawnWave1))))

(event Custom|SpawnPLayer
  (bind _returnvalue (Game|SpawnActorfromClass "/Game/SpaceShooter/BPS/P_Ship_01.P_Ship_01_C" (Math|Transform|MakeTransform "200.000000,540.000000, 0" "0, 0, 0" "1.000000,1.000000,1.000000") "Undefined" 0 0))
  (bind _output_get (Variables|Default|SetPlayerShipREF _returnvalue))
  (Variables|/Game/SpaceShooter/BPS/P_Ship_01.P_Ship_01_C|SetPlayerMovementState _output_get "NewEnumerator0")
  (Default|SetState (Variables|Default|GetPlayerShipREF))
  (Variables|/Game/SpaceShooter/BPS/P_Ship_01.P_Ship_01_C|SetPlayerMovementState _output_get "NewEnumerator2")
  (Default|SetState (Variables|Default|GetPlayerShipREF))
  (CallFunction|SpawnUI))

(event Custom|Spawn_UI
  (bind _returnvalue (Game|SpawnActorfromClass "/Game/SpaceShooter/BPS/BP_InGame_UI.BP_InGame_UI_C" (Math|Transform|MakeTransform "0, 0, 0" "0, 0, 0" "1.000000,1.000000,1.000000") "Undefined" 0 0))
  (bind _output_get (Variables|Default|SetGUI_REF _returnvalue))
  (Default|ToggleWaveVisability (Variables|/Game/SpaceShooter/BPS/BP_InGame_UI.BP_InGame_UI_C|GetW_GUI_REF _output_get))
  (Utilities|FlowControl|Delay 2.0)
  (CallFunction|LoadWave))

(event Custom|SPawn%20Wave%201
  (switch int (Variables|Default|GetSquadrenNumber)
    (:0
      (CallFunction|SpawnEnemiesonSpline "-200.000000,20.000000, 0" 10 2 "/Game/SpaceShooter/BPS/BP_EnemyMine_01.BP_EnemyMine_01_C" 8.0))
    (:1
      (CallFunction|SpawnEnemiesonSpline "-200.000000,1000.000000, 0" 10 0 "/Game/SpaceShooter/BPS/BP_EnemyMine_01.BP_EnemyMine_01_C" 8.0))
    (:2
      (CallFunction|SpawnEnemiesonSpline "-200.000000,40.000000, 0" 10 2 "/Game/SpaceShooter/BPS/BP_EnemyMine_01.BP_EnemyMine_01_C" 8.0)
      (CallFunction|SpawnEnemiesonSpline "-200.000000,1000.000000, 0" 10 0 "/Game/SpaceShooter/BPS/BP_EnemyMine_01.BP_EnemyMine_01_C" 8.0))))

(event EventBeginPlay
  (CallFunction|SpawnPLayer))

(event EventSquadrenDestroyed
  (Math|Integer|IncrementInt (Variables|Default|GetSquadrenNumber)
    (:%20%20
      (CallFunction|SPawnWave1))))

(fn ConstructionScript)

(fn SpawnEnemiesonSpline
  (params (SpawnLocation :type Vector) (NumberEnemies :type Integer) (SplineTrackSelection :type Integer) (EnemyType :type Actor%20Class%20Reference) (TimeToCompleteSpline :type Float%20%28double-precision%29))
  (bind _returnvalue (Game|SpawnActorfromClass "/Game/SpaceShooter/BPS/BP_SpawnerBase.BP_SpawnerBase_C" (Math|Transform|MakeTransform "0, 0, 0" "0, 0, 0" "1.000000,1.000000,1.000000") "Undefined" 0 0))
  (Variables|/Game/SpaceShooter/BPS/BP_SpawnerBase.BP_SpawnerBase_C|SetSpawnLocation _returnvalue SpawnLocation)
  (Variables|/Game/SpaceShooter/BPS/BP_SpawnerBase.BP_SpawnerBase_C|SetNumberEnemiesToSpawn _returnvalue NumberEnemies)
  (Variables|/Game/SpaceShooter/BPS/BP_SpawnerBase.BP_SpawnerBase_C|SetSplineSelection _returnvalue SplineTrackSelection)
  (Variables|/Game/SpaceShooter/BPS/BP_SpawnerBase.BP_SpawnerBase_C|SetEnemyClassToSpawn _returnvalue EnemyType)
  (Variables|/Game/SpaceShooter/BPS/BP_SpawnerBase.BP_SpawnerBase_C|SetSetTimeToCompleteSpline _returnvalue TimeToCompleteSpline)
  (Default|InitialCalibrationComplete _returnvalue))