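; BPC_Debug is a debug component in the SpaceShooter game that visualizes the bounds of its owning actor.
; On BeginPlay it prints the actor's box extent to the screen.
; Each Tick it draws a thick pink box for the full actor bounds, inset slightly, and a green box for the root component's bounds, allowing comparison between the two.
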(event EventBeginPlay
  (Development|PrintString (Utilities|String|ToString(Vector) (.BoxExtent (Collision|GetActorBounds (Components|GetOwner) false false))) true true "(R=0.000000,G=0.660000,B=1.000000,A=1.000000)" 1e+01))

(event EventTick
  (params (DeltaSeconds :type Float%20%28single-precision%29))
  (bind _returnvalue (Components|GetOwner))
  (bind _returnvalue_2 (Components|GetOwner))
  (bind (_origin _boxextent) (Collision|GetActorBounds _returnvalue false false))
  (bind _rootcomponent (Variables|/Script/Engine.Actor|GetRootComponent _returnvalue_2))
  (bind (_origin_2 _boxextent_2) (Collision|GetComponentBounds _rootcomponent))
  (Rendering|Debug|DrawDebugBox _origin (- _boxextent "10.000000,10.000000,10.000000") "(R=1.000000,G=0.000000,B=0.718530,A=1.000000)" "0, 0, 0" 0.0 3.0)
  (Rendering|Debug|DrawDebugBox _origin_2 _boxextent_2 "(R=0.000000,G=1.000000,B=0.067770,A=1.000000)" "0, 0, 0" 0.0 0.0))