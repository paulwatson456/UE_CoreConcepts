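; Chain gun actor for the space shooter that fires Niagara particle bullets and turns them into damaging hits.
; It registers itself as the Niagara system's export callback, then sphere-traces at the first exported particle's position.
; Blocking hits damage the actor's I_Entity_Damageable component and spawn an offset impact effect.
; Debug-style number keys 1–3 adjust bullet spawn rate, and the first two also set velocity scale.
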(event EventBeginPlay
  (bind _returnvalue (Niagara|SpawnSystemAttached "/Game/SpaceShooter/BPS/NS_GunBullets_01.NS_GunBullets_01" (Variables|Default|GetDefaultSceneRoot) "None" "0, 0, 0" "0, 0, 0" "KeepRelativeOffset" false))
  (bind _output_get (Variables|Default|SetNS_REF _returnvalue))
  (Niagara|SetNiagaraVariable(Object) _output_get "User.BP_Callback" self)
  (Input|EnableInput (Game|GetPlayerController 0)))

(event Collision|EventActorBeginOverlap
  (params (OtherActor :type Actor%20Object%20Reference)))

(event EventTick
  (params (DeltaSeconds :type Float%20%28single-precision%29)))

(event EventParticleData
  (params (Data :type Array%20of%20Basic%20Particle%20Data%20Structures) (NiagaraSystem :type Niagara%20System%20Object%20Reference) (SimulationPositionOffset :type Vector%20%28by%20ref%29 :default "0, 0, 0"))
  (bind _output (Utilities|Array|Get(acopy) Data))
  (bind _position (Utilities|Struct|BreakBasicParticleData _output))
  (bind _outhit (Collision|SphereTraceByChannel _position _position 5e+01 "TraceTypeQuery1" false 0 "None" true "(R=1.000000,G=0.000000,B=0.000000,A=1.000000)" "(R=0.000000,G=1.000000,B=0.000000,A=1.000000)" 2.0))
  (if (.bBlockingHit (Collision|BreakHitResult _outhit))
    (Class|IEntityDamageable|DamageEntityValue(Message) (Utilities|Array|Get(acopy) (Class|Actor|GetComponentsbyInterface (.HitActor (Collision|BreakHitResult _outhit)) "/Game/SpaceShooter/BPS/I_Entity_Damageable.I_Entity_Damageable_C")) 3e+01)
    (Niagara|SpawnSystematLocation "/Game/SpaceShooter/BPS/NS_GunImpact_01.NS_GunImpact_01" (+ (.Location (Collision|BreakHitResult _outhit)) "40.000000,0,0"))))

(event Input|KeyboardEvents|2
  (params (Key :type Key%20Structure :default "None"))
  (bind _ns_ref (Variables|Default|GetNS_REF))
  (:Pressed
    (Niagara|SetNiagaraVariable(Float) _ns_ref "User.SpawnRate" 1e+01)
    (Niagara|SetNiagaraVariable(Float) _ns_ref "User.VelocitySpeedScale" 1.5)))

(event Input|KeyboardEvents|3
  (params (Key :type Key%20Structure :default "None"))
  (:Pressed
    (Niagara|SetNiagaraVariable(Float) (Variables|Default|GetNS_REF) "User.SpawnRate" 2e+01)))

(event Input|KeyboardEvents|1
  (params (Key :type Key%20Structure :default "None"))
  (bind _ns_ref (Variables|Default|GetNS_REF))
  (:Pressed
    (Niagara|SetNiagaraVariable(Float) _ns_ref "User.SpawnRate" 5.0)
    (Niagara|SetNiagaraVariable(Float) _ns_ref "User.VelocitySpeedScale" 0.5)))

(fn ConstructionScript)