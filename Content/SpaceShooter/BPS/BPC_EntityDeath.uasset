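; Actor component that handles the death of an entity in the SpaceShooter game.
; On EntityDeath it reads defeat points from the owner's stats component, halts its movement component (both found by interface), and adds the points to the GameState score.
; It then notifies the spawner that a squadron unit is down and moves the owner back to the location cached on BeginPlay instead of destroying it.
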(event EventBeginPlay
  (bind _asgs_space_shooter (Utilities|Casting|CastToGS_SpaceShooter (Game|GetGameState)))
  (Variables|Default|SetAs%20GS%20Space%20Shooter _asgs_space_shooter)
  (Variables|Default|SetWorldLocationOnSpawn (Transformation|GetActorLocation (Components|GetOwner))))

(event EventTick
  (params (DeltaSeconds :type Float%20%28single-precision%29)))

(event EventEntityDeath
  (bind _returnvalue (Components|GetOwner))
  (bind _pointsondefeatbase_stat (Class|IEntitySTATS|ReturnBaseSTATS(Message) (Utilities|Array|Get(acopy) (Class|Actor|GetComponentsbyInterface (Components|GetOwner) "/Game/SpaceShooter/BPS/I_Entity_STATS.I_Entity_STATS_C"))))
  (Variables|Default|SetPointsForScore _pointsondefeatbase_stat)
  (Class|IEntityMovement|StopMovement(Message) (Utilities|Array|Get(acopy) (Class|Actor|GetComponentsbyInterface (Components|GetOwner) "/Game/SpaceShooter/BPS/I_Entity_Movement.I_Entity_Movement_C")))
  (Class|IUpdateGSData|UpdateScoreTotal(Message) (Variables|Default|GetAs%20GS%20Space%20Shooter) (Variables|Default|GetPointsForScore))
  (Class|ISpawner|SquadrenUnitDown(Message) (Variables|Default|GetSpawnerREF) (Components|GetOwner))
  (Transformation|SetActorLocation _returnvalue (Variables|Default|GetWorldLocationOnSpawn) false false)
  (Development|PrintString (Utilities|GetDisplayName _returnvalue)))