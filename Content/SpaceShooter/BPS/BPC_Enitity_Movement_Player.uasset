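; Player movement component for the space shooter that moves the owning actor's root with eased acceleration and banks it on sideways input.
; Each axis input nudges a clamped curve position that decays on release, and a direction curve turns it into a scaled speed.
; The right/left axis event applies both axes' world offset and sets roll from a rotation curve.
; Movement runs per input event without delta-time scaling.
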(event EventTick
  (params (DeltaSeconds :type Float%20%28single-precision%29)))

(event EventBeginPlay
  (Variables|Default|SetOwner%20Root%20Component (Variables|/Script/Engine.Actor|GetRootComponent (Components|GetOwner))))

(event Input|AxisEvents|InputAxisMoveRight/Left
  (params (AxisValue :type Float%20%28single-precision%29))
  (bind _initialrotation (Variables|Default|GetInitialRotation))
  (Variables|Default|SetLR_AxisValue AxisValue)
  (bind _new_lr_time_over_curve (CallFunction|LRAxistoCurveMapping (Variables|Default|GetLR_TimeOverCurve) (Variables|Default|GetLR_AxisValue) (== AxisValue 0.0)))
  (Variables|Default|SetLR_TimeOverCurve _new_lr_time_over_curve)
  (bind _lr_offset (CallFunction|ApplyCurvetoLRAccelleration (Variables|Default|GetCurveDirectionSpeed)))
  (Transformation|AddWorldOffset (Variables|/Script/Engine.Actor|GetRootComponent (Components|GetOwner)) (Math|Vector|MakeVector (stale Input|AxisEvents|InputAxisMoveForward/Backward _ud_offset) _lr_offset 0.0) false false)
  (Transformation|SetWorldRotation (Variables|Default|GetOwner%20Root%20Component) (Math|Rotator|Lerp(Rotator) "0, 0, 0" (Math|Rotator|MakeRotator (+ (.roll _initialrotation) 2e+01) (.pitch _initialrotation) (.yaw _initialrotation)) (Math|Curves|GetFloatValue (Variables|Default|GetCurveRotationSpeed) (Variables|Default|GetLR_TimeOverCurve))) false false))

(event Input|AxisEvents|InputAxisMoveForward/Backward
  (params (AxisValue :type Float%20%28single-precision%29))
  (Variables|Default|SetUD_AxisValue AxisValue)
  (bind _new_ud_time_over_curve (CallFunction|UDAxistoCurveMapping (Variables|Default|GetUD_TimeOverCurve) (Variables|Default|GetUD_AxisValue) (== AxisValue 0.0)))
  (Variables|Default|SetUD_TimeOverCurve _new_ud_time_over_curve)
  (bind _ud_offset (CallFunction|ApplyCurvetoUDAccelleration (Variables|Default|GetCurveDirectionSpeed))))

(fn LRAxistoCurveMapping
  (params (Current%20LR%20time%20over%20curve :type Float%20%28double-precision%29) (LR%20axis%20value :type Float%20%28double-precision%29) (DirectionPressed? :type Boolean))
  (if DirectionPressed?
    (Variables|Default|SetLR_TimeOverCurve (Math|Float|Clamp(Float) (- Current%20LR%20time%20over%20curve (/ Current%20LR%20time%20over%20curve 2e+01)) -1.0))
    (else
      (Variables|Default|SetLR_TimeOverCurve (Math|Float|Clamp(Float) (+ (/ LR%20axis%20value 2e+01) Current%20LR%20time%20over%20curve) -1.0))))
  (return (Variables|Default|GetLR_TimeOverCurve)))

(fn ApplyCurvetoLRAccelleration
  (params (Curve :type Curve%20Float%20Object%20Reference))
  (return (* (Math|Curves|GetFloatValue Curve (Variables|Default|GetLR_TimeOverCurve)) (Variables|Default|GetSpeedMultiplier))))

(fn UDAxistoCurveMapping
  (params (Current%20UD%20time%20over%20curve :type Float%20%28double-precision%29) (UD%20axis%20value :type Float%20%28double-precision%29) (DirectionPressed? :type Boolean))
  (if DirectionPressed?
    (Variables|Default|SetUD_TimeOverCurve (Math|Float|Clamp(Float) (- Current%20UD%20time%20over%20curve (/ Current%20UD%20time%20over%20curve 2e+01)) -1.0))
    (else
      (Variables|Default|SetUD_TimeOverCurve (Math|Float|Clamp(Float) (+ (/ UD%20axis%20value 2e+01) Current%20UD%20time%20over%20curve) -1.0))))
  (return (Variables|Default|GetUD_TimeOverCurve)))

(fn ApplyCurvetoUDAccelleration
  (params (Curve :type Curve%20Float%20Object%20Reference))
  (return (* (Math|Curves|GetFloatValue Curve (Variables|Default|GetUD_TimeOverCurve)) (Variables|Default|GetSpeedMultiplier))))