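; Projectile actor for the space shooter that flies forward and damages ships it overlaps.
; Tick moves it without sweep, easing out toward a point ahead along its forward vector with delta seconds as alpha, and a Delay on the same chain destroys it two seconds later.
; Cube overlap sends a fixed DamageMessage to the other actor's components implementing I_Ship, without destroying the bullet.
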(event OnComponentHit(Cube)
  (params (HitComponent :type Primitive%20Component%20Object%20Reference) (OtherActor :type Actor%20Object%20Reference) (OtherComp :type Primitive%20Component%20Object%20Reference) (NormalImpulse :type Vector :default "0, 0, 0") (Hit :type Hit%20Result%20Structure%20%28by%20ref%29)))

(event OnComponentBeginOverlap(Cube)
  (params (OverlappedComponent :type Primitive%20Component%20Object%20Reference) (OtherActor :type Actor%20Object%20Reference) (OtherComp :type Primitive%20Component%20Object%20Reference) (OtherBodyIndex :type Integer) (bFromSweep :type Boolean) (SweepResult :type Hit%20Result%20Structure%20%28by%20ref%29))
  (for _array_element (Class|Actor|GetComponentsbyInterface OtherActor "/Game/SpaceShooter/BPS/I_Ship.I_Ship_C")
    (Class|IShip|Damage(Message) _array_element 5.0)))

(event EventBeginPlay)

(event Collision|EventActorBeginOverlap
  (params (OtherActor :type Actor%20Object%20Reference)))

(event EventTick
  (params (DeltaSeconds :type Float%20%28single-precision%29))
  (bind _defaultsceneroot (Variables|Default|GetDefaultSceneRoot))
  (bind _returnvalue (Transformation|GetWorldLocation _defaultsceneroot))
  (Transformation|SetActorLocation (Math|Interpolation|Ease "EaseOut" DeltaSeconds _returnvalue (+ (* (Math|Vector|GetForwardVector _defaultsceneroot) 1e+03) _returnvalue) 2.0) false false)
  (Utilities|FlowControl|Delay 2.0)
  (Actor|DestroyActor))

(fn ConstructionScript)