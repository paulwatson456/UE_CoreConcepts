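; BPC_SpawnSpline is an actor component in the space shooter that adds a spline component to its owner at BeginPlay.
; It builds the spline from the first track in the PDASplineTracks data, setting the stored point locations and then each tangent in local space.
; The new spline is kept in SplineREF, and MoveObject is an empty stub, so nothing moves along the spline here.
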(event EventBeginPlay
  (bind _pda_splinetracks (Variables|Default|GetPDA_SplineTracks))
  (bind _st_splinetracks (Variables|/Game/SpaceShooter/BPS/SplineTracks/PDA_SplineTracks.PDA_SplineTracks_C|GetST_SplineTracks _pda_splinetracks))
  (bind _output (Utilities|Array|Get(acopy) _st_splinetracks))
  (bind _asspline_component (Utilities|Casting|CastToSplineComponentClass "/Script/Engine.SplineComponent"))
  (bind _returnvalue (Game|AddComponentbyClass (Components|GetOwner) _asspline_component false))
  (bind _output_get (Variables|Default|SetSplineREF _returnvalue))
  (Spline|SetSplinePoints _output_get (.pointworldlocations _output) "Local" true)
  (for (_array_element _array_index) (.pointtangents _output)
    (Spline|SetTangentatSplinePoint (Variables|Default|GetSplineREF) _array_index _array_element "Local" true)))

(fn MoveObject)