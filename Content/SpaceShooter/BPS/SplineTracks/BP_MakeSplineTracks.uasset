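; Spline authoring actor for the SpaceShooter game that records a track's shape into a data asset.
; The construction script copies each SplineTrack point's local location and tangent into arrays, clearing only the locations beforehand.
; SaveSpline appends those arrays, with track name and point count, to the PDASlpineTracks track list.
; A 1920x1080 debug box marks the play area, and PlayerContext is moved to its center during construction.
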(event EventBeginPlay
  (Rendering|Debug|DrawDebugBox "960.000000,540.000000, 0" "960.000000,540.000000, 0" "(R=0.942708,G=0.042036,B=0.000000,A=1.000000)" "0, 0, 0" 2e+01 2e+01))

(fn ConstructionScript
  (bind _spline_points_number (Variables|Default|GetSpline%20Points%20Number))
  (Utilities|Array|Clear (Variables|Default|GetSplinePointsLocation))
  (bind _output_get (Variables|Default|SetNumberOfSplinePoints (Spline|GetNumberOfSplinePoints (Variables|Default|GetSplineTrack))))
  (Utilities|Array|Resize _spline_points_number _output_get)
  (for (_ _array_index) _spline_points_number
    (Utilities|Array|Add (Variables|Default|GetSplinePointsLocation) (.location (Spline|GetTransformatSplinePoint (Variables|Default|GetSplineTrack) _array_index "Local" false)))
    (Utilities|Array|Add (Variables|Default|GetSplinePointsTangent) (Spline|GetTangentatSplinePoint (Variables|Default|GetSplineTrack) _array_index "Local"))
    (Rendering|Debug|DrawDebugBox "960.000000,540.000000, 0" "960.000000,540.000000, 0" "(R=0.942708,G=0.042036,B=0.000000,A=1.000000)" "0, 0, 0" 2e+01 2e+01)
    (Transformation|SetWorldLocation (Variables|Default|GetPlayerContext) "960.000000,540.000000, 0" false false)))

(fn SaveSpline
  (Utilities|Array|Add (Variables|/Game/SpaceShooter/BPS/SplineTracks/PDA_SplineTracks.PDA_SplineTracks_C|GetST_SplineTracks (Variables|Default|GetPDA%20SlpineTracks)) (Utilities|Struct|MakeST_SplineTracks (Variables|Default|GetTrackName) (Variables|Default|GetSplinePointsLocation) (Variables|Default|GetNumberOfSplinePoints) (Variables|Default|GetSplinePointsTangent))))