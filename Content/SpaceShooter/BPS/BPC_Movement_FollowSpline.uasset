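; Movement component for the space shooter that moves its owning actor along a referenced spline in a repeating loop.
; Tick advances a normalized progress value by time, wraps it to zero, and maps it to spline distance to set the root's world location and rotation.
; EnableMovement and StopMovement toggle only the transform update, so progress keeps advancing while the actor is stopped.
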(event EventBeginPlay)

(event EventTick
  (params (DeltaSeconds :type Float%20%28single-precision%29))
  (bind _splineref (Variables|Default|GetSplineREF))
  (bind _output_get (Variables|Default|SetZeroToOne (+ (/ DeltaSeconds (Variables|Default|GetTimeToCompleteSpline)) (Variables|Default|GetZeroToOne))))
  (if (> _output_get 1.0)
    (Variables|Default|SetZeroToOne 0.0))
  (if (Variables|Default|GetCanMove?)
    (Utilities|IsValid (Variables|Default|GetSplineREF)
      (:Is%20Valid
        (Transformation|SetWorldLocationAndRotation (Variables|/Script/Engine.Actor|GetRootComponent (Components|GetOwner)) (Spline|GetLocationatDistanceAlongSpline _splineref (Math|Float|Lerp 0.0 (Spline|GetSplineLength (Variables|Default|GetSplineREF)) (Variables|Default|GetZeroToOne)) "World") (Spline|GetRotationatDistanceAlongSpline _splineref (Math|Float|Lerp 0.0 (Spline|GetSplineLength (Variables|Default|GetSplineREF)) (Variables|Default|GetZeroToOne)) "World") false false)))))

(event EventEnableMovement
  (Variables|Default|SetCanMove? true))

(event EventStopMovement
  (Variables|Default|SetCanMove? false))