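; Actor component that gives a Space Shooter entity health, damage handling and a collision box that hurts the player.
; On BeginPlay it builds a "Damageable" box sized from the owner's padded bounds and reads max health from the owner's stats interface component.
; Damage lowers clamped health when damageable, sending a death message through the owner's death interface at zero.
; Player pawn overlap with the box sends fixed damage to the player's damageable component.
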(event Custom|OnComponentBeginOverlap_Event_0
  (params (OverlappedComponent :type Primitive%20Component%20Object%20Reference) (OtherActor :type Actor%20Object%20Reference) (OtherComp :type Primitive%20Component%20Object%20Reference) (OtherBodyIndex :type Integer) (bFromSweep :type Boolean) (SweepResult :type Hit%20Result%20Structure%20%28by%20ref%29))
  (if (== OtherActor (Game|Player|GetPlayerPawn 0))
    (Class|IEntityDamageable|DamageEntityValue(Message) (Utilities|Array|Get(acopy) (Class|Actor|GetComponentsbyInterface (Game|Player|GetPlayerPawn 0) "/Game/SpaceShooter/BPS/I_Entity_Damageable.I_Entity_Damageable_C")) 1e+02)))

(event EventDamageEntityValue
  (params (DMG_Amount :type Float%20%28double-precision%29))
  (Variables|Default|SetIncomingDamage DMG_Amount)
  (if (Variables|Default|GetIsDamageable?)
    (Variables|Default|SetHealthCurrent (Math|Float|Clamp(Float) (- (Variables|Default|GetHealthCurrent) (Variables|Default|GetIncomingDamage)) 0.0 (Variables|Default|GetHealthMax)))
    (if (<= (Variables|Default|GetHealthCurrent) 0.0)
      (Class|IEntityDeath|EntityDeath(Message) (Utilities|Array|Get(acopy) (Class|Actor|GetComponentsbyInterface (Components|GetOwner) "/Game/SpaceShooter/BPS/I_Entity_Death.I_Entity_Death_C"))))))

(event EventRemoveCollision
  (Collision|SetCollisionEnabled (Variables|Default|GetEntityCollision) "NoCollision"))

(event EventBeginPlay
  (bind _output_get (Variables|Default|SetOwnerREF (Components|GetOwner)))
  ;[1 1 1] would it be simpler to have a collider already and then adjust it? Constructing appears to require assignment of events as an extra step
  (bind _returnvalue (Game|AddComponentbyClass _output_get "/Script/Engine.BoxComponent" false (Math|Transform|MakeTransform "0, 0, 0" "0, 0, 0" (/ (+ (.BoxExtent (Collision|GetActorBounds _output_get false false)) "20.000000,20.000000,20.000000") "50.000000,50.000000,25.000000"))))
  (bind _output_get_2 (Variables|Default|SetEntityCollision _returnvalue))
  (Development|SetHiddeninGame _returnvalue true false)
  (Collision|SetCollisionProfileName _returnvalue "Damageable" false :!class /Script/Engine.PrimitiveComponent)
  ;[1 1 1] might not need this
  (Variables|/Script/Engine.ActorComponent|SetComponentTags (Variables|Default|GetEntityCollision) (Utilities|Array|MakeArray (Variables|Default|GetTagToAvoidDamage)))
  (Collision|AssignOnComponentBeginOverlap (Variables|Default|GetEntityCollision) (delegate Custom|OnComponentBeginOverlap_Event_0))
  (bind _healthbase_stat (Class|IEntitySTATS|ReturnBaseSTATS(Message) (Utilities|Array|Get(acopy) (Class|Actor|GetComponentsbyInterface (Components|GetOwner) "/Game/SpaceShooter/BPS/I_Entity_STATS.I_Entity_STATS_C"))))
  (bind _output_get_3 (Variables|Default|SetHealthMax _healthbase_stat))
  (Variables|Default|SetHealthCurrent _output_get_3))

(fn GetHealth
  (return (Variables|Default|GetHealthCurrent)))