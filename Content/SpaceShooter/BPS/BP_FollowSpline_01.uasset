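; Actor that moves a mine along a spline track rebuilt at runtime from saved data.
; On BeginPlay it adds a spline component and fills its points and tangents from the first track in the PDASplineTracks data.
; A timeline, rate-scaled by TimeToComplete, then drives the mine by distance along the spline with a fixed rotation rather than following the spline's direction.
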(event Custom|MoveObject
  (Components|Timeline|SetPlayRate (Variables|Default|GetMoveObject_TL) (/ 1.0 (Variables|Default|GetTimeToComplete)))
  (bind _movetrack (Timeline|MoveObject_TL Play)
    (:Update
      (Transformation|SetWorldLocationAndRotation (Variables|Default|GetSP_Mine_01) (Spline|GetLocationatDistanceAlongSpline (Variables|Default|GetSplineTrackREF) (Math|Float|Lerp 0.0 (Spline|GetSplineLength (Variables|Default|GetSplineTrackREF)) _movetrack) "World") "0, 0,90.000000" false false))))

(event EventBeginPlay
  (bind _pda_splinetracks (Variables|Default|GetPDA_SplineTracks))
  (bind _st_splinetracks (Variables|/Game/SpaceShooter/BPS/SplineTracks/PDA_SplineTracks.PDA_SplineTracks_C|GetST_SplineTracks _pda_splinetracks))
  (bind _output (Utilities|Array|Get(acopy) _st_splinetracks))
  ;[1 1 1] Creates Spline based on previously saved data
  (bind _returnvalue (AddComponent|AddSplineComponent false (Transformation|GetRelativeTransform (Variables|Default|GetDefaultSceneRoot))))
  (bind _output_get (Variables|Default|SetSplineTrackREF _returnvalue))
  (Spline|SetSplinePoints _output_get (.pointworldlocations _output) "Local" true)
  (for (_array_element _array_index) (.pointtangents _output)
    (Spline|SetTangentatSplinePoint (Variables|Default|GetSplineTrackREF) _array_index _array_element "World" true))
  (CallFunction|MoveObject))

(fn ConstructionScript)