(event Custom|Death
  (Utilities|FlowControl|Delay 0.2)
  (Actor|DestroyActor (Variables|Default|GetOwnerREF)))

(event EventDamage
  (params (DMG_Value :type Float%20%28double-precision%29))
  (Variables|Default|SetIncomingDamage DMG_Value)
  (if (Variables|Default|GetIsDamageable?)
    (Variables|Default|SetHealthCurrent (Math|Float|Clamp(Float) (- (Variables|Default|GetHealthCurrent) (Variables|Default|GetIncomingDamage)) 0.0 (Variables|Default|GetHealthMax)))
    (for _array_element (Class|Actor|GetComponentsbyInterface (Variables|Default|GetOwnerREF) "/Game/SpaceShooter/BPS/I_Ship.I_Ship_C")
      (Class|IShip|UpdateHealthDisplay(Message) _array_element (Variables|Default|GetHealthCurrent) (Variables|Default|GetHealthMax))
      (if (<= (Variables|Default|GetHealthCurrent) 0.0)
        (CallFunction|Death)
        (else
          (Development|PrintString (Utilities|String|ToString(Float) (Variables|Default|GetHealthCurrent))))))))

(event EventBeginPlay
  (Variables|Default|SetOwnerREF (Components|GetOwner)))

(event EventCheckStats
  (params (MaxHealth :type Float%20%28double-precision%29))
  ;[1 1 1] Gets health from parent actor
  (bind _output_get (Variables|Default|SetHealthMax MaxHealth))
  (Variables|Default|SetHealthCurrent _output_get)
  (for _array_element (Class|Actor|GetComponentsbyInterface (Variables|Default|GetOwnerREF) "/Game/SpaceShooter/BPS/I_Ship.I_Ship_C")
    (Class|IShip|UpdateHealthDisplay(Message) _array_element (Variables|Default|GetHealthCurrent) (Variables|Default|GetHealthMax))))