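; Examinable object that shows its description in an on-screen widget, one page per interaction.
; Interact drives a three-state switch: the first call creates WBP_ExaminableObject and notifies the player pawn, later calls advance through the ObjectDescription array.
; After the last page, another Interact notifies the pawn, removes the widget and resets for reuse.
; The page-count check runs only after the first page, so descriptions need at least two entries.
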(event EventBeginPlay
  (Variables|Default|SetDialoguePageLength (Utilities|Array|Length (Variables|Default|GetObjectDescription))))

(event Collision|EventActorBeginOverlap
  (params (OtherActor :type Actor%20Object%20Reference)))

(event EventTick
  (params (DeltaSeconds :type Float%20%28single-precision%29)))

(event EventInteract
  (params (KeyInventory :type Array%20of%20Strings))
  (switch Utilities|FlowControl|Switch|SwitchonE_Dialougue (Variables|Default|GetState)
    (:NewEnumerator0
      (bind _returnvalue (UserInterface|CreateWidget "/Game/States/WBP_ExaminableObject.WBP_ExaminableObject_C"))
      (bind _output_get (Variables|Default|SetObjectUI _returnvalue))
      (UserInterface|Viewport|AddtoViewport _output_get 0)
      (Class|IDialogue|DialogueStart(Message) (Game|Player|GetPlayerPawn 0))
      (Variables|Default|SetState "NewEnumerator1")
      (Rendering|Components|TextRender|SetText (Variables|/Game/States/WBP_ExaminableObject.WBP_ExaminableObject_C|GetObjectDescription (Variables|Default|GetObjectUI)) (Utilities|Array|Get(acopy) (Variables|Default|GetObjectDescription)))
      (bind _result (Math|Integer|IncrementInt (Variables|Default|GetCurrent%20Dialogue%20Page))
        (:%20%20
          (Variables|Default|SetCurrent%20Dialogue%20Page _result))))
    (:NewEnumerator1
      (Rendering|Components|TextRender|SetText (Variables|/Game/States/WBP_ExaminableObject.WBP_ExaminableObject_C|GetObjectDescription (Variables|Default|GetObjectUI)) (Utilities|Array|Get(acopy) (Variables|Default|GetObjectDescription) (Variables|Default|GetCurrent%20Dialogue%20Page)))
      (bind _result_2 (Math|Integer|IncrementInt (Variables|Default|GetCurrent%20Dialogue%20Page))
        (:%20%20
          (Variables|Default|SetCurrent%20Dialogue%20Page _result_2)
          (if (== (Variables|Default|GetCurrent%20Dialogue%20Page) (Variables|Default|GetDialoguePageLength))
            (Variables|Default|SetState "NewEnumerator2")))))
    (:NewEnumerator2
      (Class|IDialogue|DialougueEnd(Message) (Game|Player|GetPlayerPawn 0))
      (Widget|RemovefromParent (Variables|Default|GetObjectUI))
      (Variables|Default|SetState "NewEnumerator0")
      (Variables|Default|SetCurrent%20Dialogue%20Page 0))))

(fn ConstructionScript)