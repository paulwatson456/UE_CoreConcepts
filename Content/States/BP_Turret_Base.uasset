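; Base enemy camera turret that sweeps back and forth on patrol and turns to face the player on detection.
; Collapsed graphs lay out a Patrol/Alert state flow, with detection collider overlaps acting as the transitions.
; Timelines drive the cube's ping-pong yaw sweep, the looping look-at tracking, and a lerp back to the saved rotation before patrol resumes.
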(fn ConstructionScript)

(event Custom|Rotate
  (switch Utilities|FlowControl|Switch|SwitchonE_RotationDirection (Variables|Default|GetE_Rotation)
    (:NewEnumerator0
      (bind _newtrack_0 (Timeline|Rotation Play)
        (:Update
          (Transformation|SetRelativeRotation (Variables|Default|GetCube) (Math|Rotator|MakeRotator 0.0 0.0 _newtrack_0) false false))
        (:Finished
          (Utilities|FlowControl|FlipFlop
            (:A
              (Variables|Default|SetE_Rotation "NewEnumerator1"))
            (:B
              (Variables|Default|SetE_Rotation "NewEnumerator0")))
          (CallFunction|Rotate))))
    (:NewEnumerator1
      (Timeline|Rotation Reverse))))

(event Custom|PausePatrol
  (bind _newtrack_0 (Timeline|Rotation Stop)
    (:Update
      (Transformation|SetRelativeRotation (Variables|Default|GetCube) (Math|Rotator|MakeRotator 0.0 0.0 _newtrack_0) false false))
    (:Finished
      (Utilities|FlowControl|FlipFlop
        (:A
          (Variables|Default|SetE_Rotation "NewEnumerator1"))
        (:B
          (Variables|Default|SetE_Rotation "NewEnumerator0")))
      (CallFunction|Rotate))))

(event OnComponentBeginOverlap(DetectionCollider)
  (params (OverlappedComponent :type Primitive%20Component%20Object%20Reference) (OtherActor :type Actor%20Object%20Reference) (OtherComp :type Primitive%20Component%20Object%20Reference) (OtherBodyIndex :type Integer) (bFromSweep :type Boolean) (SweepResult :type Hit%20Result%20Structure%20%28by%20ref%29))
  (if (== OtherActor (Game|Player|GetPlayerPawn 0))
    (Development|PrintString "Hello")
    (Variables|Default|SetStartROT (Variables|/Script/Engine.SceneComponent|GetRelativeRotation (Variables|Default|GetCube)))
    (CallFunction|PausePatrol)
    (CallFunction|StopReset)
    (CallFunction|AlertTrackPlayer)
    (else
      (Development|PrintString "You are not my enemy"))))

(event Custom|StopTrackingPlayer
  (Timeline|TrackPlayerUpdate Stop
    (:Update
      (Transformation|SetRelativeRotation (Variables|Default|GetCube) (Math|Rotator|MakeRotator 0.0 0.0 (.yaw (Math|Rotator|FindLookatRotation (Transformation|GetWorldLocation (Variables|Default|GetCube)) (Transformation|GetWorldLocation (Variables|/Script/Engine.Actor|GetRootComponent (Game|Player|GetPlayerPawn 0)))))) false false))
    (:Finished
      (CallFunction|AlertTrackPlayer))))

(event Custom|AlertTrackPlayer
  (Timeline|TrackPlayerUpdate PlayFromStart
    (:Update
      (Transformation|SetRelativeRotation (Variables|Default|GetCube) (Math|Rotator|MakeRotator 0.0 0.0 (.yaw (Math|Rotator|FindLookatRotation (Transformation|GetWorldLocation (Variables|Default|GetCube)) (Transformation|GetWorldLocation (Variables|/Script/Engine.Actor|GetRootComponent (Game|Player|GetPlayerPawn 0)))))) false false))
    (:Finished
      (CallFunction|AlertTrackPlayer))))

(event OnComponentEndOverlap(DetectionCollider)
  (params (OverlappedComponent :type Primitive%20Component%20Object%20Reference) (OtherActor :type Actor%20Object%20Reference) (OtherComp :type Primitive%20Component%20Object%20Reference) (OtherBodyIndex :type Integer))
  (if (== OtherActor (Game|Player|GetPlayerPawn 0))
    (Development|PrintString "GoodBye")
    (CallFunction|StopTrackingPlayer)
    (CallFunction|ResettoPatrolRotation)))

(event Custom|StopReset
  (bind _newtrack_0 (Timeline|Timeline_0 Stop)
    (:Update
      (Transformation|SetRelativeRotation (Variables|Default|GetCube) (Math|Rotator|Lerp(Rotator) (Variables|/Script/Engine.SceneComponent|GetRelativeRotation (Variables|Default|GetCube)) (Variables|Default|GetStartROT) _newtrack_0) false false))
    (:Finished
      (CallFunction|Rotate))))

(event Custom|ResetToPatrolRotation
  (bind _newtrack_0 (Timeline|Timeline_0 PlayFromStart)
    (:Update
      (Transformation|SetRelativeRotation (Variables|Default|GetCube) (Math|Rotator|Lerp(Rotator) (Variables|/Script/Engine.SceneComponent|GetRelativeRotation (Variables|Default|GetCube)) (Variables|Default|GetStartROT) _newtrack_0) false false))
    (:Finished
      (CallFunction|Rotate))))

(event EventBeginPlay
  (CallFunction|Rotate)
  (return))