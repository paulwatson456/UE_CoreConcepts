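; Base Blueprint for a key-locked door that swings open and shut when interacted with.
; Interact checks the passed key inventory for KeyNeeded, sets an Open or Closed state, and dispatches to that state's event.
; OpenFunctionality uses a FlipFlop to alternate DoorPivot between rotated and unrotated over a short move at its starting location.
; ClosedFunctionality only prints a locked message, alongside debug text naming the missing key.
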(event Custom|ClosedFunctionality
  (Development|PrintString "I am Locked"))

(event Custom|OpenFunctionality
  (Utilities|FlowControl|FlipFlop
    (:A
      (Components|MoveComponentTo (Variables|Default|GetDoorPivot) (Variables|Default|GetStartingLocation) "0,90.000000, 0" false false 0.5 false))
    (:B
      (Components|MoveComponentTo (Variables|Default|GetDoorPivot) (Variables|Default|GetStartingLocation) "0,0.000000, 0" false false 0.5 false))))

(event EventInteract
  (params (KeyInventory :type Array%20of%20Strings))
  (if (Utilities|Array|ContainsItem KeyInventory (Variables|Default|GetKeyNeeded))
    (Variables|Default|SetState "NewEnumerator0")
    (Development|PrintString "Key Found")
    (else
      (Variables|Default|SetState "NewEnumerator1")
      (Development|PrintString (Utilities|String|Append (Variables|Default|GetKeyNeeded) " needed to unlock me"))))
  (switch Utilities|FlowControl|Switch|SwitchonE_OpenClose (Variables|Default|GetState)
    (:NewEnumerator0
      (CallFunction|OpenFunctionality))
    (:NewEnumerator1
      (CallFunction|ClosedFunctionality))))

(event EventBeginPlay
  (Variables|Default|SetState "NewEnumerator1")
  (Variables|Default|SetStartingLocation (Variables|/Script/Engine.SceneComponent|GetRelativeLocation (Variables|Default|GetDoorPivot))))

(fn ConstructionScript)